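; Game mode that spawns the player at the PlayerStart named by the SpawnPoint stored in TheGameInstance.
; BeginPlay caches the game instance and destroys any existing player character, printing a red error if the cast fails.
; Tick restarts the player at that named start whenever no valid character exists, and otherwise prints SpawnPoint on screen each frame as debug output.
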(event EventTick
  (params (DeltaSeconds :type Float%20%28single-precision%29))
  (Utilities|IsValid (Game|GetPlayerCharacter 0)
    (:Is%20Valid
      (Development|PrintString (Variables|/Game/Blueprints/TheGameInstance.TheGameInstance_C|GetSpawnPoint (Variables|Default|GetGameInstance)) true true "(R=0.000000,G=0.660000,B=1.000000,A=1.000000)" 0.0))
    (:Is%20Not%20Valid
      (Class|GameModeBase|RestartPlayeratPlayerStart (Game|GetPlayerController 0) (Class|GameModeBase|FindPlayerStart 0 (Variables|/Game/Blueprints/TheGameInstance.TheGameInstance_C|GetSpawnPoint (Variables|Default|GetGameInstance)))))))

(event EventBeginPlay
  (bind _returnvalue (Game|GetPlayerCharacter 0))
  (bind _asthe_game_instance (Utilities|Casting|CastToTheGameInstance (Game|GetGameInstance))
    (:then
      (Variables|Default|SetGameInstance _asthe_game_instance)
      (Utilities|IsValid _returnvalue
        (:Is%20Valid
          (Actor|DestroyActor _returnvalue))))
    (:CastFailed
      (Development|PrintString "EH SOMETHING WRONG 
" true true "(R=1.000000,G=0.000000,B=0.000000,A=1.000000)" 4.0))))

(fn ConstructionScript)