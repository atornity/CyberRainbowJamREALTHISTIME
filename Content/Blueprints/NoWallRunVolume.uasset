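; NoWallRunVolume is a volume that prevents characters from wall running while inside it.
; It stores the overlapping BaseCharacter on begin overlap and clears it when that actor leaves.
; Every tick it checks the stored character and calls DetachFromWall if that character is wall running.
; Only one character is tracked at a time, with the latest to enter replacing any earlier one.
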(event EventBeginPlay)

(event Collision|EventActorBeginOverlap
  (params (OtherActor :type Actor%20Object%20Reference))
  (bind _asbase_character (Utilities|Casting|CastToBaseCharacter OtherActor))
  (Variables|Default|SetOverlappedActor _asbase_character))

(event EventTick
  (params (DeltaSeconds :type Float%20%28single-precision%29))
  (bind _overlappedactor (Variables|Default|GetOverlappedActor))
  (Utilities|IsValid _overlappedactor
    (:Is%20Valid
      (if (Variables|/Game/Blueprints/3dBaseCharacter.BaseCharacter_C|GetWallRunning _overlappedactor)
        (Default|DetachfromWall (Variables|Default|GetOverlappedActor))))))

(event Collision|EventActorEndOverlap
  (params (OtherActor :type Actor%20Object%20Reference))
  (if (== OtherActor (Variables|Default|GetOverlappedActor))
    (Variables|Default|SetOverlappedActor 0)))

(fn ConstructionScript)