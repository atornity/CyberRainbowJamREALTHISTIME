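; Climbable stairs actor that works like a ladder for an overlapping BaseCharacter, with collision box and mesh sized from StairsHeight.
; Each tick it disables wall running; pushing toward it from the ground launches the character slightly into falling.
; While falling, gravity is zeroed, position eases onto the Arrow's vertical axis, and input along the actor's forward axis drives climb velocity.
; Leaving the overlap restores gravity and wall running.
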(event EventBeginPlay)

(event Collision|EventActorBeginOverlap
  (params (OtherActor :type Actor%20Object%20Reference))
  (bind _asbase_character (Utilities|Casting|CastToBaseCharacter OtherActor))
  (Variables|Default|SetCharacter _asbase_character))

(event EventTick
  (params (DeltaSeconds :type Float%20%28single-precision%29))
  (bind _returnvalue (Transformation|GetActorUpVector))
  (bind _character (Variables|Default|GetCharacter))
  (bind _character_2 (Variables|Default|GetCharacter))
  (bind _arrow (Variables|Default|GetArrow))
  (bind _character_3 (Variables|Default|GetCharacter))
  (bind _character_4 (Variables|Default|GetCharacter))
  (bind _returnvalue_2 (Transformation|GetActorLocation _character_2))
  (bind _returnvalue_3 (Transformation|GetWorldLocation _arrow))
  (bind (_return _returnvalue_4) (Default|GetMovementInput _character))
  (bind _charactermovement (Variables|/Script/Engine.Character|GetCharacterMovement _character_4))
  (Utilities|IsValid _character_2
    (:Is%20Valid
      (Variables|/Game/Blueprints/3dBaseCharacter.BaseCharacter_C|SetCanWallRun _character_2 false)
      (if (AI|Components|NavMovement|IsFalling (Variables|/Script/Engine.Character|GetCharacterMovement _character_2))
        (Transformation|SetActorLocation _character_2 (Math|Interpolation|VInterpTo (Transformation|GetActorLocation (Variables|Default|GetCharacter)) (+ (- _returnvalue_2 (Math|Vector|ProjectVectorontoPlane _returnvalue_2 (Transformation|GetActorUpVector))) (- _returnvalue_3 (* _returnvalue (Math|Vector|DotProduct _returnvalue_3 _returnvalue)))) DeltaSeconds 15.0) true false)
        (Variables|/Script/Engine.MovementComponent|SetVelocity _charactermovement (Math|Interpolation|VInterpTo (Transformation|GetVelocity _character_4) (* (Transformation|GetActorUpVector) (* (Math|Vector|DotProduct (.ReturnValue (Default|GetMovementInput (Variables|Default|GetCharacter))) (* (Transformation|GetActorForwardVector) -1.0)) (Variables|Default|GetClimbSpeed))) (Utilities|Time|GetWorldDeltaSeconds) 15.0))
        (Variables|/Script/Engine.CharacterMovementComponent|SetGravityScale _charactermovement 0.0)
        (elif (and _return (> (Math|Vector|DotProduct _returnvalue_4 (* (Transformation|GetActorForwardVector) -1.0)) 0.5))
          (Character|LaunchCharacter _character_3 _returnvalue false false)
          (Variables|/Script/Engine.CharacterMovementComponent|SetGravityScale (Variables|/Script/Engine.Character|GetCharacterMovement _character_3) 1.0))))))

(event Collision|EventActorEndOverlap
  (params (OtherActor :type Actor%20Object%20Reference))
  (if (== OtherActor (Variables|Default|GetCharacter))
    (Variables|/Script/Engine.CharacterMovementComponent|SetGravityScale (Variables|/Script/Engine.Character|GetCharacterMovement (Variables|Default|GetCharacter)) 1.0)
    (Variables|/Game/Blueprints/3dBaseCharacter.BaseCharacter_C|SetCanWallRun (Variables|Default|GetCharacter) true)
    (Variables|Default|SetCharacter 0)))

(fn ConstructionScript
  (bind _stairsheight (Variables|Default|GetStairsHeight))
  (Components|Box|SetBoxExtent (Variables|Default|GetBox) (Math|Vector|MakeVector 15.0 35.0 (* _stairsheight 1e+02)) true)
  (Transformation|SetRelativeScale3D (Variables|Default|GetCube) (Math|Vector|MakeVector 0.0625 0.5 (* _stairsheight 2.0))))