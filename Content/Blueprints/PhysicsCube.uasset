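; PhysicsCube is an actor that fakes physical tipping by rotating in response to an actor overlapping it.
; Each Tick, the overlapping actor's local position relative to the box extent drives interpolated pitch and yaw, followed by a blend toward a configurable rotation offset.
; With no overlap, pitch and roll ease back to the BeginPlay rotation, and a gate opened after a short delay lets the full rotation, including yaw, recover.
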(event EventBeginPlay
  (Variables|Default|SetStartRotation (Transformation|GetActorRotation)))

(event Collision|EventActorBeginOverlap
  (params (OtherActor :type Actor%20Object%20Reference))
  (Variables|Default|SetOverlappingActor OtherActor))

(event EventTick
  (params (DeltaSeconds :type Float%20%28single-precision%29))
  (bind _returnvalue (Transformation|GetActorRotation))
  (bind _returnvalue_2 (Transformation|GetActorTransform))
  (bind _returnvalue_3 (Transformation|GetActorScale3D))
  (bind _returnvalue_4 (Transformation|GetActorRotation))
  (bind _returnvalue_5 (Transformation|GetActorRotation))
  (bind _overlappingactor (Variables|Default|GetOverlappingActor))
  (bind _box (Variables|Default|GetBox))
  (bind _startrotation (Variables|Default|GetStartRotation))
  (bind _startrotation_2 (Variables|Default|GetStartRotation))
  (bind _returnvalue_6 (Transformation|GetActorLocation _overlappingactor))
  (bind (_roll _pitch) (Math|Rotator|BreakRotator _startrotation))
  (bind _boxextent (Variables|/Script/Engine.BoxComponent|GetBoxExtent _box))
  (bind _returnvalue_7 (Math|Transform|InverseTransformLocation _returnvalue_2 _returnvalue_6))
  (bind _returnvalue_8 (* _returnvalue_3 _boxextent))
  (bind _returnvalue_9 (/ _returnvalue_7 _returnvalue_8))
  (bind (_x _y) (Math|Vector|BreakVector _returnvalue_9))
  (Utilities|IsValid (Variables|Default|GetOverlappingActor)
    (:Is%20Valid
      (Transformation|SetActorRotation (Math|Interpolation|RInterpTo (Math|Rotator|MakeRotator (.roll _returnvalue_5) (.pitch _returnvalue_5) (.yaw _returnvalue_5)) (Math|Rotator|MakeRotator (.roll _returnvalue_5) (+ (.pitch _startrotation_2) (* _x (Variables|Default|GetPhysicsStuff))) (Math|Interpolation|FInterpTo (.yaw (Transformation|GetActorRotation)) (+ (.yaw _startrotation_2) (* _x (* _y -5.0))) DeltaSeconds 5.0)) DeltaSeconds 3.0))
      (Transformation|SetActorRotation (Math|Interpolation|RInterpTo (Math|Rotator|MakeRotator (.roll _returnvalue) (.pitch _returnvalue) (.yaw _returnvalue)) (Math|Rotator|CombineRotators (Math|Rotator|MakeRotator (.roll _returnvalue) (.pitch _returnvalue) (.yaw (Variables|Default|GetStartRotation))) (Variables|Default|GetRotateWhenPlayerIsOnForThisAmmount)) DeltaSeconds 1.0))
      (goto _label Close))
    (:Is%20Not%20Valid
      (Transformation|SetActorRotation (Math|Interpolation|RInterpTo _returnvalue_4 (Math|Rotator|MakeRotator _roll _pitch (.Yaw (Math|Rotator|BreakRotator _returnvalue_4))) DeltaSeconds 2.0))
      (Utilities|FlowControl|Sequence
        (:then_0
          (Utilities|FlowControl|Gate true :!label _label
            (:Exit
              (Transformation|SetActorRotation (Math|Interpolation|RInterpTo (Transformation|GetActorRotation) (Variables|Default|GetStartRotation) DeltaSeconds 1.0)))))
        (:then_1
          (Utilities|FlowControl|Delay 1.0)
          (goto _label Open))))))

(event Collision|EventActorEndOverlap
  (params (OtherActor :type Actor%20Object%20Reference))
  (Variables|Default|SetOverlappingActor 0))

(fn ConstructionScript)