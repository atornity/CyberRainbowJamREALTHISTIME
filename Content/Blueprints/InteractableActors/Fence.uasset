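; Interactable fence actor that swings around an adjustable pivot to a set target rotation once it is interacted with.
; The construction script moves the Scene pivot and Targetrotation component to Rotationpoint, keeps the Cube at the actor's location, and applies the configured rotation to the target.
; Interaction sets a flag that lets Tick ease the pivot toward that target with RInterpTo, with no reset in this graph.
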(event EventOnInteract
  (Variables|Default|SetYes true))

(event EventTick
  (params (DeltaSeconds :type Float%20%28single-precision%29))
  (bind _scene (Variables|Default|GetScene))
  (if (Variables|Default|GetYes)
    (Transformation|SetWorldRotation _scene (Math|Interpolation|RInterpTo (Transformation|GetWorldRotation _scene) (Transformation|GetWorldRotation (Variables|Default|GetTargetrotation)) DeltaSeconds 5.0) false false)))

(fn ConstructionScript
  (bind _rotationpoint (Variables|Default|GetRotationpoint))
  (bind _targetrotation (Variables|Default|GetTargetrotation))
  (|CallParentFunction)
  (Transformation|SetRelativeLocation (Variables|Default|GetScene) _rotationpoint false false)
  (Transformation|SetWorldLocation (Variables|Default|GetCube) (Transformation|GetActorLocation) false false)
  (Transformation|SetRelativeLocation _targetrotation _rotationpoint false false)
  (Transformation|SetRelativeRotation _targetrotation (Variables|Default|GetRotateok) false false))