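; An interactable actor that travels the player to another level when used.
; On interact it opens the level named by LevelName, then writes its PlayerStartTag into the SpawnPoint of TheGameInstance.
; The game instance carries that tag across the level change, presumably to pick the player start in the new level.
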(event EventBeginPlay
  (|CallParentFunction) ; This node is disabled and will not be called.\nDrag off pins to build functionality.
)

(event Collision|EventActorBeginOverlap
  (params (OtherActor :type Actor%20Object%20Reference))
  (|CallParentFunction OtherActor) ; This node is disabled and will not be called.\nDrag off pins to build functionality.
)

(event EventTick
  (params (DeltaSeconds :type Float%20%28single-precision%29))
  (|CallParentFunction DeltaSeconds) ; This node is disabled and will not be called.\nDrag off pins to build functionality.
)

(event EventOnInteract
  (Game|OpenLevel(byName) (Variables|Default|GetLevelName))
  (bind _asthe_game_instance (Utilities|Casting|CastToTheGameInstance (Game|GetGameInstance)))
  (Variables|/Game/Blueprints/TheGameInstance.TheGameInstance_C|SetSpawnPoint _asthe_game_instance (Variables|Default|GetPlayerStartTag)))

(fn ConstructionScript
  (|CallParentFunction))