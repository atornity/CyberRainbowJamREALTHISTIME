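; Actor component that lets a BaseCharacter find and interact with SwitchActors in view.
; Each tick it sphere-traces from the spring arm along control rotation, with debug drawing and component tag prints.
; GetHit picks one hit by plane-projected distance and sets a widget location halfway between impact point and trace line.
; Interact calls the cached switch while the trace reports a hit.
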(event Custom|Interact
  (bind _interactableactor (Variables|Default|GetInteractableActor))
  (if (Variables|Default|GetWidgetActive)
    (Utilities|IsValid _interactableactor
      (:Is%20Valid
        (Default|Interact _interactableactor)))))

(event EventTick
  (params (DeltaSeconds :type Float%20%28single-precision%29))
  (bind _basecharacter (Variables|Default|GetBaseCharacter))
  (bind _returnvalue (Pawn|GetControlRotation _basecharacter :!class /Script/Engine.Pawn))
  (bind _springarm (Variables|/Game/Blueprints/3dBaseCharacter.BaseCharacter_C|GetSpringArm _basecharacter))
  (bind _returnvalue_2 (Math|Vector|GetForwardVector _returnvalue))
  (bind _returnvalue_3 (Transformation|GetWorldLocation _springarm))
  (bind (_outhits _returnvalue_4) (Collision|MultiSphereTraceByChannel _returnvalue_3 (+ _returnvalue_3 (* _returnvalue_2 (Variables|Default|GetInteractDistance))) (Variables|Default|GetInteractRadius) "TraceTypeQuery3" false 0 "ForOneFrame"))
  (bind _output_get (Variables|Default|SetWidgetActive _returnvalue_4))
  (if _output_get
    (bind _output_get_2 (Variables|Default|SetWidgetDistance (.Distance (CallFunction|GetHit _outhits _returnvalue_2 _returnvalue_3))))
    (Variables|Default|SetWidgetLocation (.WidgetLocation (CallFunction|GetHit _outhits _returnvalue_2 _returnvalue_3)))
    (bind _output_get_3 (Variables|Default|SetWidgetTags (Variables|/Script/Engine.ActorComponent|GetComponentTags (.HitComponent (Collision|BreakHitResult (.Hit (CallFunction|GetHit _outhits _returnvalue_2 _returnvalue_3)))))))
    (for _array_element _output_get_3
      (Development|PrintString (Utilities|String|ToString(Name) _array_element) true true "(R=0.000000,G=0.660000,B=1.000000,A=1.000000)" 0.0))
    (bind _asswitch_actor (Utilities|Casting|CastToSwitchActor (.HitActor (Collision|BreakHitResult (.Hit (CallFunction|GetHit _outhits _returnvalue_2 _returnvalue_3))))))
    (Variables|Default|SetInteractableActor _asswitch_actor)))

(event EventBeginPlay
  (bind _asbase_character (Utilities|Casting|CastToBaseCharacter (Components|GetOwner)))
  (Variables|Default|SetBaseCharacter _asbase_character))

(fn GetHit
  (params (Array :type Array%20of%20Hit%20Result%20Structures) (PlaneNormal :type Vector) (Location :type Vector))
  (for (_array_element _array_index) Array
    (if (or (== _array_index 0) (< (Math|Vector|Distance(Vector) (Math|Vector|ProjectVectorontoPlane (.ImpactPoint (Collision|BreakHitResult _array_element)) PlaneNormal) (Math|Vector|ProjectVectorontoPlane PlaneNormal Location)) (LocalVariables|GetBestDistance)))
      (LocalVariables|SetBestDistance (Math|Vector|Distance(Vector) (Math|Vector|ProjectVectorontoPlane (.ImpactPoint (Collision|BreakHitResult _array_element)) PlaneNormal) (Math|Vector|ProjectVectorontoPlane PlaneNormal Location)))
      (LocalVariables|SetT _array_element)))
  (return (.bBlockingHit (Collision|BreakHitResult (LocalVariables|GetT))) (LocalVariables|GetT) (Math|Vector|Lerp(Vector) (.ImpactPoint (Collision|BreakHitResult (LocalVariables|GetT))) (+ Location (* (Math|Vector|GetUnitDirection(Vector) (.TraceStart (Collision|BreakHitResult (LocalVariables|GetT))) (.TraceEnd (Collision|BreakHitResult (LocalVariables|GetT)))) (Math|Vector|DotProduct (- (.ImpactPoint (Collision|BreakHitResult (LocalVariables|GetT))) (.TraceStart (Collision|BreakHitResult (LocalVariables|GetT)))) (Math|Vector|GetUnitDirection(Vector) (.TraceStart (Collision|BreakHitResult (LocalVariables|GetT))) (.TraceEnd (Collision|BreakHitResult (LocalVariables|GetT))))))) 0.5) (LocalVariables|GetBestDistance)))