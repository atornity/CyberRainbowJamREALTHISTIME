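; Interactable actor that activates an InterpToMovement component on interact to move along designer-defined control points.
; The construction script places and scales the Cube mesh at the first point and copies the points and duration into the movement component.
; It also spawns a duplicate DebugMesh at the last point as a destination preview, which BeginPlay destroys.
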(event EventBeginPlay
  (|CallParentFunction)
  (Components|DestroyComponent (Variables|Default|GetDebugMesh)))

(event Collision|EventActorBeginOverlap
  (params (OtherActor :type Actor%20Object%20Reference))
  (|CallParentFunction OtherActor) ; This node is disabled and will not be called.\nDrag off pins to build functionality.
)

(event EventTick
  (params (DeltaSeconds :type Float%20%28single-precision%29))
  (|CallParentFunction DeltaSeconds) ; This node is disabled and will not be called.\nDrag off pins to build functionality.
)

(event EventOnInteract
  (Components|Activation|SetActive (Variables|Default|GetInterpToMovement) true false))

(fn ConstructionScript
  (bind _interptomovement (Variables|Default|GetInterpToMovement))
  (bind _cube (Variables|Default|GetCube))
  (bind _cube_2 (Variables|Default|GetCube))
  (|CallParentFunction)
  (Transformation|SetRelativeLocation _cube_2 (.PositionControlPoint (Utilities|Struct|BreakInterpControlPoint (Utilities|Array|Get(acopy) (Variables|Default|GetControlPoints)))) false false)
  (Transformation|SetRelativeScale3D _cube_2 (Variables|Default|GetMeshScale))
  (bind _output_get (Variables|/Script/Engine.InterpToMovementComponent|SetControlPoints _interptomovement (Variables|Default|GetControlPoints)))
  (Variables|/Script/Engine.InterpToMovementComponent|SetDuration _interptomovement (Variables|Default|GetDuration))
  (bind _returnvalue (AddComponent|AddStaticMeshComponent false (Transformation|GetRelativeTransform _cube)))
  (bind _output_get_2 (Variables|Default|SetDebugMesh _returnvalue))
  (Components|StaticMesh|SetStaticMesh _output_get_2 (Variables|/Script/Engine.StaticMeshComponent|GetStaticMesh _cube))
  (Transformation|SetRelativeLocation (Variables|Default|GetDebugMesh) (.PositionControlPoint (Utilities|Struct|BreakInterpControlPoint (Utilities|Array|Get(acopy) _output_get (Utilities|Array|LastIndex (Variables|Default|GetControlPoints))))) false false))