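; SwitchActor is an overlap-triggered switch that drives other InteractableActors sharing its InteractTag.
; Any actor beginning overlap calls Interact, which sets Interacted and calls OnInteract on every matching actor; ending overlap calls UnInteract, which calls StopInteract on them.
; Targets are found through GetAllActorsOfClass on each call, and UnInteract leaves Interacted set.
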(event EventBeginPlay)

(event Collision|EventActorBeginOverlap
  (params (OtherActor :type Actor%20Object%20Reference))
  (CallFunction|Interact))

(event EventTick
  (params (DeltaSeconds :type Float%20%28single-precision%29)))

(event Collision|EventActorEndOverlap
  (params (OtherActor :type Actor%20Object%20Reference))
  (CallFunction|UnInteract))

(fn ConstructionScript)

(fn Interact
  (Variables|Default|SetInteracted true)
  (bind _outactors (Actor|GetAllActorsOfClass "/Game/Blueprints/InteractableActors/InteractableActor.InteractableActor_C"))
  (for _array_element _outactors
    (if (Utilities|Enum|Equal(Enum) (Variables|/Game/Blueprints/InteractableActors/InteractableActor.InteractableActor_C|GetInteractTag _array_element) (Variables|Default|GetInteractTag))
      (Default|OnInteract _array_element))))

(fn UnInteract
  (bind _outactors (Actor|GetAllActorsOfClass "/Game/Blueprints/InteractableActors/InteractableActor.InteractableActor_C"))
  (for _array_element _outactors
    (if (Utilities|Enum|Equal(Enum) (Variables|/Game/Blueprints/InteractableActors/InteractableActor.InteractableActor_C|GetInteractTag _array_element) (Variables|Default|GetInteractTag))
      (Default|StopInteract _array_element))))