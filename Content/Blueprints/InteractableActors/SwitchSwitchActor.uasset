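; SwitchSwitchActor is an interactable actor with a configurable Cube mesh component whose tags reflect its Interacted state.
; The construction script applies mesh, material, scale, in-game visibility and collision, either blocking or overlapping pawns, and starts with the not-interacted tags.
; Every Tick it rewrites the component's tags from the interacted or not-interacted set by polling Interacted, which this graph never sets.
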(event EventBeginPlay)

(event EventTick
  (params (DeltaSeconds :type Float%20%28single-precision%29))
  (CallFunction|SetCompTags (select (Variables|Default|GetInteracted) (Variables|Default|GetInteractedTags) (Variables|Default|GetNotInteractedTags))))

(fn ConstructionScript
  (bind _cube (Variables|Default|GetCube))
  (bind _enablecollission (Variables|Default|GetEnableCollission))
  (bind _cube_2 (Variables|Default|GetCube))
  (Variables|/Script/Engine.ActorComponent|SetComponentTags (Variables|Default|GetCube) (Variables|Default|GetNotInteractedTags))
  (Transformation|SetRelativeScale3D _cube (Variables|Default|GetMeshScale))
  (Rendering|Material|SetMaterial _cube 0 (Variables|Default|GetMeshMaterial))
  (Components|StaticMesh|SetStaticMesh _cube (Variables|Default|GetMesh))
  (Development|SetHiddeninGame _cube_2 (Variables|Default|GetHiddenInGame) false)
  (Collision|SetCollisionEnabled _cube_2 (select _enablecollission "QueryAndPhysics" "QueryOnly"))
  (Collision|SetCollisionResponsetoChannel (Variables|Default|GetCube) "ECC_Pawn" (select _enablecollission "ECR_Block" "ECR_Overlap")))

(fn SetCompTags
  (params (ComponentTags :type Array%20of%20Names))
  (Variables|/Script/Engine.ActorComponent|SetComponentTags (Variables|Default|GetCube) ComponentTags))