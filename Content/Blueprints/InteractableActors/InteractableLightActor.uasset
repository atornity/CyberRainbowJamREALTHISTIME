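; An interactable light actor that switches its point light on and off in response to interaction.
; OnInteract shows the PointLight and StopInteract hides it, each printing a debug string.
; The construction script applies the LightColor variable to the light, so the color is set per instance before play.
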(event EventBeginPlay
  (|CallParentFunction) ; This node is disabled and will not be called.\nDrag off pins to build functionality.
)

(event Collision|EventActorBeginOverlap
  (params (OtherActor :type Actor%20Object%20Reference))
  (|CallParentFunction OtherActor) ; This node is disabled and will not be called.\nDrag off pins to build functionality.
)

(event EventTick
  (params (DeltaSeconds :type Float%20%28single-precision%29))
  (|CallParentFunction DeltaSeconds))

(event EventOnInteract
  ;[1 1 1] interact
  (Rendering|SetVisibility (Variables|Default|GetPointLight) true false)
  (Development|PrintString "Interact"))

(event EventStopInteract
  ;[1 1 1] Comment
  (Rendering|SetVisibility (Variables|Default|GetPointLight) false false)
  (Development|PrintString "StopInteract"))

(fn ConstructionScript
  (|CallParentFunction)
  (Rendering|Components|Light|SetLightColor (Variables|Default|GetPointLight) (Variables|Default|GetLightColor) true))